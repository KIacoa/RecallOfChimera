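; Player Blueprint for a card-and-grid game, holding health, stamina and monster variations, with an M key music toggle.
; A looping timer drives hover detection, tracing along Y under the cursor in Game stage to toggle card, monster and special-spot detail popups.
; Stat changes are clamped and refresh the character HUD, with stamina locked while S001LeftRound is active.
; Death opens the settlement widget and switches the stage, mirrored on the controller, to UI.
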(event Custom|HoverDetect
  (bind _returnvalue (Game|GetPlayerController 0))
  (bind _gamemanager (Variables|Default|GetGameManager))
  (bind _worldlocation (Game|Player|ConvertMouseLocationToWorldSpace _returnvalue))
  (bind _wbp_game (Variables|/Game/Resource/BP/GameManager/BP_GameManager.BP_GameManager_C|GetWBP_Game _gamemanager))
  (bind (_x _y _z) (Math|Vector|BreakVector _worldlocation))
  (bind (_x_2 _y_2 _z_2) (Math|Vector|BreakVector _worldlocation))
  (switch Utilities|FlowControl|Switch|SwitchonE_Stage (Variables|Default|GetStage)
    (:NewEnumerator1
      (bind (_outhit _returnvalue_2) (Collision|LineTraceByChannel (Math|Vector|MakeVector _x 5e+01 _z) (Math|Vector|MakeVector _x_2 -5e+01 _z_2) "TraceTypeQuery1" false 0 "None"))
      (if _returnvalue_2
        (Utilities|FlowControl|Sequence
          (:then_0
            (bind _asbp_card (Utilities|Casting|CastToBP_Card (.HitActor (Collision|BreakHitResult _outhit)))
              (:then
                (Utilities|FlowControl|Sequence
                  (:then_0
                    (if (not (Variables|/Game/Resource/BP/Card/BP_Card.BP_Card_C|GetIsBack _asbp_card))
                      (Default|Show/HideCardDetail (Variables|/Game/Resource/BP/GameManager/BP_GameManager.BP_GameManager_C|GetWBP_Game (Variables|Default|GetGameManager)) true (Math|Vector2D|MakeVector2D (+ (.x (.ScreenPosition (Class|WidgetLayoutLibrary|ProjectWorldLocationtoWidgetPosition (Variables|Default|GetAs%20BP%20Player%20Controller) (Transformation|GetActorLocation _asbp_card) false))) 75.0) (- (.y (.ScreenPosition (Class|WidgetLayoutLibrary|ProjectWorldLocationtoWidgetPosition (Variables|Default|GetAs%20BP%20Player%20Controller) (Transformation|GetActorLocation _asbp_card) false))) 157.0)) (Variables|/Game/Resource/BP/Card/BP_Card.BP_Card_C|GetCardID _asbp_card))
                      (else
                        (Default|Show/HideCardDetail :self (Variables|/Game/Resource/BP/GameManager/BP_GameManager.BP_GameManager_C|GetWBP_Game (Variables|Default|GetGameManager)) :!label _label))))))
              (:CastFailed
                (goto _label))))
          (:then_1
            (bind _asbp_grid_monster (Utilities|Casting|CastToBP_GridMonster (.HitActor (Collision|BreakHitResult _outhit)))
              (:then
                (Default|Show/HideMonsterDetail (Variables|/Game/Resource/BP/GameManager/BP_GameManager.BP_GameManager_C|GetWBP_Game (Variables|Default|GetGameManager)) true (Math|Vector2D|MakeVector2D (- (.x (.ScreenPosition (Class|WidgetLayoutLibrary|ProjectWorldLocationtoWidgetPosition (Variables|Default|GetAs%20BP%20Player%20Controller) (Transformation|GetActorLocation _asbp_grid_monster) false))) 175.0) (+ (.y (.ScreenPosition (Class|WidgetLayoutLibrary|ProjectWorldLocationtoWidgetPosition (Variables|Default|GetAs%20BP%20Player%20Controller) (Transformation|GetActorLocation _asbp_grid_monster) false))) 2e+01)) (Variables|/Game/Resource/BP/Grid/Monster/BP_GridMonster.BP_GridMonster_C|GetMonsterID _asbp_grid_monster)))
              (:CastFailed
                (Default|Show/HideMonsterDetail (Variables|/Game/Resource/BP/GameManager/BP_GameManager.BP_GameManager_C|GetWBP_Game (Variables|Default|GetGameManager)) false (Math|Vector2D|MakeVector2D 0.0 0.0) "None"))))
          (:then_2
            (bind _asbp_grid_special_spot (Utilities|Casting|CastToBP_GridSpecialSpot (.HitActor (Collision|BreakHitResult _outhit)))
              (:then
                (Default|Show/HideSpecialSpotDetail (Variables|/Game/Resource/BP/GameManager/BP_GameManager.BP_GameManager_C|GetWBP_Game (Variables|Default|GetGameManager)) true (Math|Vector2D|MakeVector2D (- (.x (.ScreenPosition (Class|WidgetLayoutLibrary|ProjectWorldLocationtoWidgetPosition (Variables|Default|GetAs%20BP%20Player%20Controller) (Transformation|GetActorLocation _asbp_grid_special_spot) false))) 1.6e+02) (+ (.y (.ScreenPosition (Class|WidgetLayoutLibrary|ProjectWorldLocationtoWidgetPosition (Variables|Default|GetAs%20BP%20Player%20Controller) (Transformation|GetActorLocation _asbp_grid_special_spot) false))) 2e+01)) (Variables|/Game/Resource/BP/Grid/Special/BP_GridSpecialSpot.BP_GridSpecialSpot_C|GetSpotID _asbp_grid_special_spot)))
              (:CastFailed
                (Default|Show/HideSpecialSpotDetail (Variables|/Game/Resource/BP/GameManager/BP_GameManager.BP_GameManager_C|GetWBP_Game (Variables|Default|GetGameManager)) false (Math|Vector2D|MakeVector2D 0.0 0.0) "None")))))
        (else
          (Default|Show/HideCardDetail :self _wbp_game)
          (Default|Show/HideMonsterDetail :self _wbp_game)
          (Default|Show/HideSpecialSpotDetail :self _wbp_game))))))

(event EventBeginPlay
  (|CallParentFunction)
  (bind _asbp_player_controller (Utilities|Casting|CastToBP_PlayerController (Game|GetPlayerController 0)))
  (Variables|Default|SetAs%20BP%20Player%20Controller _asbp_player_controller)
  (CallFunction|ChangeStage "NewEnumerator1")
  (Utilities|Time|SetTimerbyEvent (EventDispatchers|CreateEvent :!event Custom|HoverDetect) 0.2 true))

(event Collision|EventActorBeginOverlap
  (params (OtherActor :type Actor%20Object%20Reference)))

(event EventTick
  (params (DeltaSeconds :type Float%20%28single-precision%29)))

(event Game|Damage|EventAnyDamage
  (params (Damage :type Float%20%28single-precision%29) (DamageType :type Damage%20Type%20Object%20Reference) (InstigatedBy :type Controller%20Object%20Reference) (DamageCauser :type Actor%20Object%20Reference))
  (CallFunction|ChangeHealth (* Damage -1.0))
  (Utilities|FlowControl|Sequence
    (:then_0
      (bind _gamemanager (Variables|Default|GetGameManager)
        (:then
          (Default|SetHealth/Stamina (Variables|/Game/Resource/BP/WBP/Game/WBP_Game.WBP_Game_C|GetWBP_Character (Variables|/Game/Resource/BP/GameManager/BP_GameManager.BP_GameManager_C|GetWBP_Game _gamemanager)) true))
        (:else)))
    (:then_1
      (if (<= (Variables|Default|GetHealth) 0.0)
        (CallFunction|Die)))))

(event Input|KeyboardEvents|M
  (params (Key :type Key%20Structure :default "None"))
  (bind _gamemanager (Variables|Default|GetGameManager))
  (bind _as_bp_game_instance (Variables|/Game/Resource/BP/GameManager/BP_GameManager.BP_GameManager_C|GetAs%20BP%20Game%20Instance _gamemanager))
  (bind _musicvolume (Variables|/Game/Resource/BP/GameMode/BP_GameInstance.BP_GameInstance_C|GetMusicVolume _as_bp_game_instance))
  (bind _returnvalue (== _musicvolume 0.0))
  (:Pressed
    (Default|AdjustMusicVolume (Variables|/Game/Resource/BP/GameManager/BP_GameManager.BP_GameManager_C|GetAs%20BP%20Game%20Instance (Variables|Default|GetGameManager)) (select _returnvalue 0.7 0.0))
    (if _returnvalue
      (Default|PlayBackgroundMusic (Variables|/Game/Resource/BP/GameManager/BP_GameManager.BP_GameManager_C|GetAs%20BP%20Game%20Instance (Variables|Default|GetGameManager)) "/Game/Resource/Assets/Sound/BGM/SE_GamePlay_1.SE_GamePlay_1" 0.7))))

(fn ConstructionScript
  (|CallParentFunction))

(fn AddVariation
  (params (Monster :type Name))
  (bind _variations (Variables|Default|GetVariations))
  (if (== (Utilities|Array|FindItem _variations Monster) -1)
    (Utilities|Array|AddUnique _variations Monster)
    (CallFunction|ExecuteVariationEffect Monster)
    (Default|SetPlayerImage (Variables|/Game/Resource/BP/WBP/Game/WBP_Game.WBP_Game_C|GetWBP_Character (Variables|/Game/Resource/BP/GameManager/BP_GameManager.BP_GameManager_C|GetWBP_Game (Variables|Default|GetGameManager))))))

(fn ChangeStamina
  (params (Value :type Integer))
  (LocalVariables|SetOriginalStamina (Variables|Default|GetStamina))
  (if (not (> (Variables|Default|GetS_001LeftRound) 0))
    (Variables|Default|SetStamina (Math|Integer|Clamp(Integer) (+ Value (Variables|Default|GetStamina)) 0 (Variables|Default|GetStaminaMax)))
    (bind _gamemanager (Variables|Default|GetGameManager)
      (:then
        (Default|SetHealth/Stamina (Variables|/Game/Resource/BP/WBP/Game/WBP_Game.WBP_Game_C|GetWBP_Character (Variables|/Game/Resource/BP/GameManager/BP_GameManager.BP_GameManager_C|GetWBP_Game _gamemanager)) false))
      (:else
        _))
    (return (- (Variables|Default|GetStamina) (LocalVariables|GetOriginalStamina)))))

(fn ChangeHealth
  (params (Value :type Float%20%28double-precision%29))
  (LocalVariables|SetOriginalHealth (Variables|Default|GetHealth))
  (Variables|Default|SetHealth (Math|Float|Clamp(Float) (+ (Variables|Default|GetHealth) Value) 0.0 (Variables|Default|GetHealthMax)))
  (bind _gamemanager (Variables|Default|GetGameManager)
    (:then
      (Default|SetHealth/Stamina (Variables|/Game/Resource/BP/WBP/Game/WBP_Game.WBP_Game_C|GetWBP_Character (Variables|/Game/Resource/BP/GameManager/BP_GameManager.BP_GameManager_C|GetWBP_Game _gamemanager)) true))
    (:else
      _))
  (return (- (Variables|Default|GetHealth) (LocalVariables|GetOriginalHealth))))

(fn Init
  (bind _output_get (Variables|Default|SetHealthMax 6.0))
  (bind _output_get_2 (Variables|Default|SetStaminaMax 8))
  (CallFunction|ChangeStamina _output_get_2)
  (CallFunction|ChangeHealth _output_get))

(fn ExecuteVariationEffect
  (params (Selection :type Name))
  (switch name Selection))

(fn ChangeStage
  (params (Stage :type E_Stage%20Enum :default "NewEnumerator0"))
  (bind _output_get (Variables|Default|SetStage Stage))
  (Variables|/Game/Resource/BP/GameMode/BP_PlayerController.BP_PlayerController_C|SetStage (Variables|Default|GetAs%20BP%20Player%20Controller) _output_get))

(fn Die
  (bind _returnvalue (UserInterface|CreateWidget "/Game/Resource/BP/WBP/Settlement/WBP_Settlement.WBP_Settlement_C"))
  (UserInterface|Viewport|AddtoViewport _returnvalue 0)
  (CallFunction|ChangeStage "NewEnumerator2"))