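; BP_Card is a pooled, clickable two-sided card for a matching mechanic, configured from DT_Card by ID.
; Clicking flips it 180 degrees via a timeline, then registers it with BP_GameManager as a special or normal card.
; Consecutive same-ID normal cards trigger an effect at TriggerCount; a mismatch flips active normals back.
; Triggering returns active normals and applies special-card modifiers, though most effect logic is unfinished.
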(event OnClicked(PaperSpriteFront)
  (params (TouchedComponent :type Primitive%20Component%20Object%20Reference) (ButtonPressed :type Key%20Structure :default "None"))
  (CallFunction|Flip))

(event OnClicked(PaperSpriteBack)
  (params (TouchedComponent :type Primitive%20Component%20Object%20Reference) (ButtonPressed :type Key%20Structure :default "None"))
  (CallFunction|Flip))

(event Custom|Flip
  (bind _gamemanager (Variables|Default|GetGameManager))
  (if (Variables|Default|GetIsActive)
    (if (not (Variables|Default|GetIsFlipping))
      (Variables|Default|SetCurrentRotation (Transformation|GetActorRotation))
      (Variables|Default|SetIsFlipping true)
      (bind _新建轨道_0 (Timeline|CardFlipTimeline PlayFromStart)
        (:Update
          (Transformation|SetActorRotation (Math|Rotator|MakeRotator (.roll (Variables|Default|GetCurrentRotation)) (.pitch (Variables|Default|GetCurrentRotation)) (Math|Float|Lerp (.yaw (Variables|Default|GetCurrentRotation)) (+ (.yaw (Variables|Default|GetCurrentRotation)) 1.8e+02) _新建轨道_0))))
        (:Finished
          (Variables|Default|SetIsFlipping false)
          (bind _output_get (Variables|Default|SetIsBack (not (Variables|Default|GetIsBack))))
          (if _output_get
            (Utilities|Array|RemoveItem (select (Variables|Default|GetIsUnique) (Variables|/Game/Resource/BP/GameManager/BP_GameManager.BP_GameManager_C|GetActiveSpecialCards (Variables|Default|GetGameManager)) (Variables|/Game/Resource/BP/GameManager/BP_GameManager.BP_GameManager_C|GetActiveNormalCards (Variables|Default|GetGameManager))) self)
            (elif (Variables|Default|GetIsUnique)
              (Utilities|Array|Add (Variables|/Game/Resource/BP/GameManager/BP_GameManager.BP_GameManager_C|GetActiveSpecialCards (Variables|Default|GetGameManager)) self)
              (elif (== (Variables|/Game/Resource/BP/GameManager/BP_GameManager.BP_GameManager_C|GetCurrentCardID (Variables|Default|GetGameManager)) "")
                (Variables|/Game/Resource/BP/GameManager/BP_GameManager.BP_GameManager_C|SetCurrentCardID _gamemanager (Variables|Default|GetCardID))
                (Variables|/Game/Resource/BP/GameManager/BP_GameManager.BP_GameManager_C|SetCurrentSameCardCount _gamemanager 1)
                (Variables|Default|SetIsActive false)
                (Utilities|Array|Add (Variables|/Game/Resource/BP/GameManager/BP_GameManager.BP_GameManager_C|GetActiveNormalCards _gamemanager) self)
                (elif (== (Variables|Default|GetCardID) (Variables|/Game/Resource/BP/GameManager/BP_GameManager.BP_GameManager_C|GetCurrentCardID (Variables|Default|GetGameManager)))
                  (bind _result (Math|Integer|IncrementInt (Variables|/Game/Resource/BP/GameManager/BP_GameManager.BP_GameManager_C|GetCurrentSameCardCount (Variables|Default|GetGameManager)))
                    (:%20%20
                      (Variables|Default|SetIsActive false)
                      (Utilities|Array|Add (Variables|/Game/Resource/BP/GameManager/BP_GameManager.BP_GameManager_C|GetActiveNormalCards (Variables|Default|GetGameManager)) self)
                      (if (== _result (Variables|Default|GetTriggerCount))
                        (CallFunction|ExecuteCardEffect))))
                  (else
                    (Variables|Default|SetIsActive false)
                    (Utilities|Array|Add (Variables|/Game/Resource/BP/GameManager/BP_GameManager.BP_GameManager_C|GetActiveNormalCards (Variables|Default|GetGameManager)) self)
                    (Default|FlipActiveNormalCards (Variables|Default|GetGameManager))))))))))))

(event EventBeginPlay
  (bind _returnvalue (Actor|GetActorOfClass "/Game/Resource/BP/GameManager/BP_GameManager.BP_GameManager_C"))
  (Variables|Default|SetGameManager _returnvalue))

(event Collision|EventActorBeginOverlap
  (params (OtherActor :type Actor%20Object%20Reference)))

(event EventTick
  (params (DeltaSeconds :type Float%20%28single-precision%29)))

(event EventOnPooledDestroy)

(event EventOnPooledSpawn
  (Variables|Default|SetIsBack true)
  (Variables|Default|SetIsActive true))

(fn ConstructionScript)

(fn Init
  (params (CardID :type Name))
  (bind _output_get (Variables|Default|SetCardID CardID))
  (bind _returnvalue (Utilities|GetDataTableRow "/Game/Resource/BP/Card/DT_Card.DT_Card" _output_get)
    (:then
      (Rendering|Components|Sprite|SetSprite (Variables|Default|GetPaperSpriteFront) (.CardSprite (Utilities|Struct|BreakST_Card _returnvalue)))
      (Variables|Default|SetIsUnique (.IsSpecial (Utilities|Struct|BreakST_Card _returnvalue)))
      (Variables|Default|SetTriggerCount (.TriggerCount (Utilities|Struct|BreakST_Card _returnvalue)))
      (Variables|Default|SetStamina%20Cost (.StaminaCost (Utilities|Struct|BreakST_Card _returnvalue))))))

(fn ExecuteCardEffect
  (Default|ReturnActiveNormalCards (Variables|Default|GetGameManager))
  (for _array_element (Variables|/Game/Resource/BP/GameManager/BP_GameManager.BP_GameManager_C|GetActiveSpecialCards (Variables|Default|GetGameManager))
    (CallFunction|ExecuteSpecialCardEffect (Variables|BP_Card_C|GetCardID _array_element)))
  (switch name (Variables|Default|GetCardID)))

(fn ExecuteSpecialCardEffect
  (params (Selection :type Name))
  (switch name Selection
    (:C_101
      (if (== (Variables|Default|GetCardID) "C_002")
        (Variables|/Game/Resource/Character/Player/BP_Player.BP_Player_C|SetIsC_101 (Variables|/Game/Resource/BP/GameManager/BP_GameManager.BP_GameManager_C|GetAs%20BP%20Player (Variables|Default|GetGameManager)) true)))
    (:C_102
      (if (or (== (Variables|Default|GetCardID) "C_001") (== (Variables|Default|GetCardID) "C_002"))
        _))))