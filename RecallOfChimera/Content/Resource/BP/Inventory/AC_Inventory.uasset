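; Inventory component that stores owned cards as counts per ID and builds a randomized card list from them.
; AddCard adds to a card's count in the AllCards map.
; RefreshCards expands the map into a count-weighted pool, then draws randomly with replacement while the result is smaller than the pool.
; Each draw adds copies per the DT_Card row's TriggerCount, capped by the room left under MaxCardCount.
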(event EventBeginPlay)

(event EventTick
  (params (DeltaSeconds :type Float%20%28single-precision%29)))

(fn AddCard
  (params (CardID :type Name) (Count :type Integer))
  (bind _allcards (Variables|Default|GetAllCards))
  (bind (_value _returnvalue) (Utilities|Map|Find _allcards CardID))
  (Utilities|Map|Add (Variables|Default|GetAllCards) CardID (select _returnvalue (+ Count _value) Count)))

(fn RefreshCards
  (LocalVariables|SetCurrentCardCount 0)
  (Utilities|Array|Clear (Variables|Default|GetCards))
  (Utilities|Array|Clear (LocalVariables|GetTempCards))
  (bind _keys (Utilities|Map|Keys (Variables|Default|GetAllCards)))
  (for _array_element _keys
    (for _index (range 1 (.Value (Utilities|Map|Find (Variables|Default|GetAllCards) _array_element)))
      (Utilities|Array|Add (LocalVariables|GetTempCards) _array_element)))
  (while (< (LocalVariables|GetCurrentCardCount) (Utilities|Array|Length (LocalVariables|GetTempCards)))
    (bind _returnvalue (Utilities|GetDataTableRow "/Game/Resource/BP/Card/DT_Card.DT_Card" (.OutItem (Utilities|Array|Random (LocalVariables|GetTempCards))))
      (:then
        (for _index_2 (range 1 (Math|Integer|Min(Integer) (.TriggerCount (Utilities|Struct|BreakST_Card _returnvalue)) (- (Variables|Default|GetMaxCardCount) (LocalVariables|GetCurrentCardCount))))
          (Utilities|Array|Add (Variables|Default|GetCards) (.CardID (Utilities|Struct|BreakST_Card _returnvalue)))
          (Math|Integer|IncrementInt (LocalVariables|GetCurrentCardCount))))))
  (return (Variables|Default|GetCards)))