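; Player controller for a card game that uses a fixed camera actor and lets the player click cards to flip them.
; On BeginPlay it adds the default Enhanced Input mapping context and switches the view to the level's BP_Camera.
; During the Game stage, a click traces along the Y axis at the deprojected mouse X/Z position and calls Flip on any BP_Card hit.
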(event Input|EnhancedActionEvents|EnhancedInputActionIA_Click
  (params (ActionValue :type Boolean) (ElapsedSeconds :type Float%20%28double-precision%29) (TriggeredSeconds :type Float%20%28double-precision%29) (InputAction :type Input%20Action%20Object%20Reference :default "/Game/Resource/Input/Actions/IA_Click.IA_Click"))
  (bind _worldlocation (Game|Player|ConvertMouseLocationToWorldSpace))
  (bind (_x _y _z) (Math|Vector|BreakVector _worldlocation))
  (bind (_x_2 _y_2 _z_2) (Math|Vector|BreakVector _worldlocation))
  (switch Utilities|FlowControl|Switch|SwitchonE_Stage (Variables|Default|GetStage)
    (:NewEnumerator1
      (bind _outhit (Collision|LineTraceByChannel (Math|Vector|MakeVector _x 5e+01 _z) (Math|Vector|MakeVector _x_2 -5e+01 _z_2) "TraceTypeQuery1" false 0 "None"))
      (bind _asbp_card (Utilities|Casting|CastToBP_Card (.HitActor (Collision|BreakHitResult _outhit))))
      (Default|Flip _asbp_card))))

(event EventBeginPlay
  (bind _returnvalue (PlayerController|LocalPlayerSubsystems|GetEnhancedInputLocalPlayerSubsystem))
  (Utilities|IsValid _returnvalue
    (:Is%20Valid
      (Input|AddMappingContext _returnvalue "/Game/Resource/Input/IMC_Default.IMC_Default" 0 "(bIgnoreAllPressedKeysUntilRelease=True,bForceImmediately=False,bNotifyUserSettings=False)")
      (bind _returnvalue_2 (Actor|GetActorOfClass "/Game/Resource/Character/Player/BP_Camera.BP_Camera_C"))
      (bind _output_get (Variables|Default|SetGameCamera _returnvalue_2))
      (Game|Player|SetViewTargetwithBlend _output_get 0.0 "VTBlend_Linear" 0.0 false))))

(event EventTick
  (params (DeltaSeconds :type Float%20%28single-precision%29)))

(fn ConstructionScript)