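; BP_GridSpecialSpot is a pooled grid actor for a special spot, with its type chosen at random.
; On each pooled spawn, after the parent logic, it picks a random row from DT_SpecialSpot, stores that row's SpotID and applies its sprite to the SpecialSpot component.
; BeginPlay, overlap and Tick are disabled stubs, and the construction script only calls the parent.
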(event EventBeginPlay
  (|CallParentFunction) ; 此节点被禁用，将不会被调用。\n从引脚连出引线来编译功能。
)

(event Collision|EventActorBeginOverlap
  (params (OtherActor :type Actor%20Object%20Reference))
  (|CallParentFunction OtherActor) ; 此节点被禁用，将不会被调用。\n从引脚连出引线来编译功能。
)

(event EventTick
  (params (DeltaSeconds :type Float%20%28single-precision%29))
  (|CallParentFunction DeltaSeconds) ; 此节点被禁用，将不会被调用。\n从引脚连出引线来编译功能。
)

(event EventOnPooledSpawn
  (|CallParentFunction)
  (bind _outrownames (DataTable|GetDataTableRowNames "/Game/Resource/BP/Grid/Special/DT_SpecialSpot.DT_SpecialSpot"))
  (bind _returnvalue (Utilities|GetDataTableRow "/Game/Resource/BP/Grid/Special/DT_SpecialSpot.DT_SpecialSpot" (.OutItem (Utilities|Array|Random _outrownames)))
    (:then
      (Variables|Default|SetSpotID (.SpotID (Utilities|Struct|BreakST_SpecialSpot _returnvalue)))
      (Rendering|Components|Sprite|SetSprite (Variables|Default|GetSpecialSpot) (.SpotSprite (Utilities|Struct|BreakST_SpecialSpot _returnvalue))))))

(fn ConstructionScript
  (|CallParentFunction))