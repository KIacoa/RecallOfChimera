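; Game manager for a card-driven adventure: creates the game UI, seeds the player's inventory from DT_Card and lays out cards and a row of map tiles.
; Cards and tiles come from an object pool, with tile types picked by DataTable weights.
; Move shifts tiles past the player's fixed slot, appends a random one, refills inactive cards and triggers spot or monster encounters.
; It also resolves monster attacks, including spell reflection, and logs story text to the UI.
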(event Custom|PlayMusic
  (Default|PlayBackgroundMusic (Variables|Default|GetAs%20BP%20Game%20Instance) "/Game/Resource/Assets/Sound/BGM/SE_GamePlay_1.SE_GamePlay_1" 0.7))

(event EventBeginPlay
  (Utilities|FlowControl|Sequence
    (:then_0
      (bind _asbp_game_instance (Utilities|Casting|CastToBP_GameInstance (Game|GetGameInstance)))
      (Variables|Default|SetAs%20BP%20Game%20Instance _asbp_game_instance)
      (bind _returnvalue (UserInterface|CreateWidget "/Game/Resource/BP/WBP/Game/WBP_Game.WBP_Game_C"))
      (bind _output_get (Variables|Default|SetWBP_Game _returnvalue))
      (UserInterface|Viewport|AddtoViewport _output_get 0)
      (bind _returnvalue_2 (UserInterface|CreateWidget "/Game/Resource/BP/WBP/WBP_Load.WBP_Load_C"))
      (UserInterface|Viewport|AddtoViewport _returnvalue_2 0)
      (EventDispatchers|BindEventtoFinishLoad _returnvalue_2 (delegate Custom|PlayMusic)))
    (:then_1
      (bind _asbp_player (Utilities|Casting|CastToBP_Player (Game|GetPlayerCharacter 0)))
      (bind _output_get_2 (Variables|Default|SetAs%20BP%20Player _asbp_player))
      (Utilities|FlowControl|Delay 0.2)
      (Default|Init _output_get_2))
    (:then_2
      (CallFunction|Init))
    (:then_3
      (Utilities|FlowControl|Delay 0.2)
      (bind _outrownames (DataTable|GetDataTableRowNames "/Game/Resource/BP/Card/DT_Card.DT_Card"))
      (for _array_element _outrownames
        (Default|AddCard (Variables|/Game/Resource/Character/Player/BP_Player.BP_Player_C|GetAC_Inventory (Variables|Default|GetAs%20BP%20Player)) _array_element 1))
      (CallFunction|RefreshAllCards)
      (CallFunction|RefreshAllGrids)
      (Variables|Default|SetStory "")
      (CallFunction|SetStory))))

(event Collision|EventActorBeginOverlap
  (params (OtherActor :type Actor%20Object%20Reference)))

(event EventTick
  (params (DeltaSeconds :type Float%20%28single-precision%29)))

(fn ConstructionScript)

(fn Init
  (Utilities|FlowControl|Sequence
    (:then_0
      (bind _returnvalue (Actor|GetActorOfClass "/Game/Resource/BP/GameManager/ObjectPool/BP_ObjectPoolManager.BP_ObjectPoolManager_C"))
      (Variables|Default|SetObjectPoolManager _returnvalue)
      (bind _returnvalue_2 (Actor|GetActorOfClass "/Game/Resource/BP/Card/BP_CardLocationSpot.BP_CardLocationSpot_C"))
      (Utilities|IsValid _returnvalue_2
        (:Is%20Valid
          (Variables|Card|SetFirstCardLocation (Transformation|GetActorLocation _returnvalue_2)))
        (:Is%20Not%20Valid
          _))
      (bind _returnvalue_3 (Actor|GetActorOfClass "/Game/Resource/BP/Grid/BP_GridLocationSpot.BP_GridLocationSpot_C"))
      (Utilities|IsValid _returnvalue_3
        (:Is%20Valid
          (Variables|Cell|SetFirstGridLocation (Transformation|GetActorLocation _returnvalue_3)))))
    (:then_2
      (CallFunction|InitGrid))))

(fn RefreshAllCards
  (bind _firstcardlocation (Variables|Card|GetFirstCardLocation))
  (for _array_element (Variables|Card|GetCards)
    (Default|ReturnObjecttoPool (Variables|Default|GetObjectPoolManager) _array_element)
    (Variables|/Game/Resource/BP/Card/BP_Card.BP_Card_C|SetIsActive _array_element false))
  (Utilities|Array|Clear (Variables|Card|GetCards))
  (bind _cards (Default|RefreshCards (Variables|/Game/Resource/Character/Player/BP_Player.BP_Player_C|GetAC_Inventory (Variables|Default|GetAs%20BP%20Player))))
  (for (_array_element_2 _array_index) _cards
    (bind _actor (Default|GetObjectfromPool (Variables|Default|GetObjectPoolManager) "/Game/Resource/BP/Card/BP_Card.BP_Card_C" (Math|Vector|MakeVector (+ (* (/ _array_index (Variables|Card|GetCardRow)) 210) (.x _firstcardlocation)) (.y _firstcardlocation) (- (.z _firstcardlocation) (* (Math|Integer|%(Integer) _array_index (Variables|Card|GetCardRow)) 300))) "0, 0, 0"))
    (bind _asbp_card (Utilities|Casting|CastToBP_Card _actor))
    (Utilities|Array|Add (Variables|Card|GetCards) _asbp_card)
    (Default|Init _asbp_card _array_element_2)))

(fn GetRandomCard
  (bind _cardid (Default|GetRandomCard (Variables|/Game/Resource/Character/Player/BP_Player.BP_Player_C|GetAC_Inventory (Variables|Default|GetAs%20BP%20Player))))
  (return _cardid))

(fn ReturnActiveNormalCards
  (Variables|Card|SetCurrentSameCardCount 0)
  (Variables|Card|SetCurrentCardID "None")
  (for _array_element (Variables|Card|GetActiveNormalCards)
    (Default|ReturnObjecttoPool (Variables|Default|GetObjectPoolManager) _array_element)
    (Variables|/Game/Resource/BP/Card/BP_Card.BP_Card_C|SetIsActive _array_element false))
  (Utilities|Array|Clear (Variables|Card|GetActiveNormalCards)))

(fn ReturnActiveSpecialCards
  (for _array_element (Variables|Card|GetActiveSpecialCards)
    (Default|ReturnObjecttoPool (Variables|Default|GetObjectPoolManager) _array_element)
    (Variables|/Game/Resource/BP/Card/BP_Card.BP_Card_C|SetIsActive _array_element false))
  (Utilities|Array|Clear (Variables|Card|GetActiveSpecialCards)))

(fn FlipActiveNormalCards
  (Variables|Card|SetCurrentSameCardCount 0)
  (Variables|Card|SetCurrentCardID "None")
  (for _array_element (Variables|Card|GetActiveNormalCards)
    (Variables|/Game/Resource/BP/Card/BP_Card.BP_Card_C|SetIsCanFlip _array_element true)
    (Default|Flip _array_element)))

(fn CompleteCards
  (bind _firstcardlocation (Variables|Card|GetFirstCardLocation))
  (for _index (range 0 (- (Variables|/Game/Resource/BP/Inventory/AC_Inventory.AC_Inventory_C|GetMaxCardCount (Variables|/Game/Resource/Character/Player/BP_Player.BP_Player_C|GetAC_Inventory (Variables|Default|GetAs%20BP%20Player))) 1))
    (if (not (Variables|/Game/Resource/BP/Card/BP_Card.BP_Card_C|GetIsActive (Utilities|Array|Get(acopy) (Variables|Card|GetCards) _index)))
      (bind _randomcardid (CallFunction|GetRandomCard))
      (bind _actor (Default|GetObjectfromPool (Variables|Default|GetObjectPoolManager) "/Game/Resource/BP/Card/BP_Card.BP_Card_C" (Math|Vector|MakeVector (+ (* (/ _index (Variables|Card|GetCardRow)) 210) (.x _firstcardlocation)) (.y _firstcardlocation) (- (.z _firstcardlocation) (* (Math|Integer|%(Integer) _index (Variables|Card|GetCardRow)) 300))) "0, 0, 0"))
      (bind _asbp_card (Utilities|Casting|CastToBP_Card _actor))
      (Utilities|Array|SetArrayElem (Variables|Card|GetCards) _index _asbp_card)
      (Default|Init _asbp_card _randomcardid))))

(fn InitGrid
  (Utilities|Array|Clear (Variables|Cell|GetAllGridTypes))
  (Utilities|Array|Clear (Variables|Cell|GetAllGridTypeWeights))
  (bind _enumvalue (|ForEachE_GridType)
    (:LoopBody
      (Utilities|Array|AddUnique (Variables|Cell|GetAllGridTypes) _enumvalue)
      (bind _returnvalue (Utilities|GetDataTableRow "/Game/Resource/BP/Grid/DT_GridType.DT_GridType" (Utilities|String|StringToName (Utilities|String|EnumtoString _enumvalue)))
        (:then
          (Utilities|Array|Add (Variables|Cell|GetAllGridTypeWeights) (.GridTypeWeight (Utilities|Struct|BreakST_GridType _returnvalue))))))))

(fn RefreshAllGrids
  (bind _firstgridlocation (Variables|Cell|GetFirstGridLocation))
  (bind _firstgridlocation_2 (Variables|Cell|GetFirstGridLocation))
  (for _array_element (Variables|Cell|GetGrids)
    (Default|ReturnObjecttoPool (Variables|Default|GetObjectPoolManager) _array_element))
  (Utilities|Array|Clear (Variables|Cell|GetGrids))
  (for _index (range 1 (Variables|Cell|GetMaxGridCount))
    (Utilities|FlowControl|Sequence
      (:then_0
        (if (<= _index 3)
          (bind _actor (Default|GetObjectfromPool (Variables|Default|GetObjectPoolManager) "/Game/Resource/BP/Grid/Path/BP_GridPath.BP_GridPath_C" (Math|Vector|MakeVector (+ (* (- _index 1) 210) (.x _firstgridlocation)) (.y _firstgridlocation) (.z _firstgridlocation)) "0, 0, 0"))
          (bind _asbp_grid (Utilities|Casting|CastToBP_Grid _actor))
          (Variables|/Game/Resource/BP/Grid/BP_Grid.BP_Grid_C|SetE_GridType _asbp_grid "NewEnumerator0")
          (Utilities|Array|Add (Variables|Cell|GetGrids) _asbp_grid)
          (else
            (bind _asbp_grid_2 (CallFunction|SpawnRandomGrid (Math|Vector|MakeVector (+ (* (- _index 1) 210) (.x _firstgridlocation)) (.y _firstgridlocation) (.z _firstgridlocation))))
            (Utilities|Array|Add (Variables|Cell|GetGrids) _asbp_grid_2))))
      (:then_1
        (if (== (- _index 1) (Variables|Default|GetPlayerSpot))
          (Transformation|SetActorLocation (Variables|Default|GetAs%20BP%20Player) (Math|Vector|MakeVector (+ (+ (* (- _index 1) 200) (.x _firstgridlocation_2)) 1e+02) (.y _firstgridlocation_2) (+ (.z _firstgridlocation_2) 5e+01)) false false))))))

(fn GetRandomGridType
  (bind _allgridtypes (Variables|Cell|GetAllGridTypes))
  (for _array_element (Variables|Cell|GetAllGridTypeWeights)
    (LocalVariables|SetTotalWeight (+ _array_element (LocalVariables|GetTotalWeight))))
  (LocalVariables|SetTempWeight (Math|Random|RandomFloatinRange 0.0 (LocalVariables|GetTotalWeight)))
  (bind (_array_element_2 _array_index) (Utilities|Array|ForEachLoopwithBreak (Variables|Cell|GetAllGridTypeWeights))
    (:LoopBody
      (bind _output_get (LocalVariables|SetTotalWeight (- (LocalVariables|GetTotalWeight) _array_element_2)))
      (if (>= (LocalVariables|GetTempWeight) _output_get)
        (return (Utilities|Array|Get(acopy) (Variables|Cell|GetAllGridTypes) _array_index))))
    (:Completed
      (return (Utilities|Array|Get(acopy) _allgridtypes (Utilities|Array|LastIndex _allgridtypes))))))

(fn SpawnRandomGrid
  (params (Location :type Vector))
  (bind _e_gridtype (CallFunction|GetRandomGridType))
  (LocalVariables|SetTempGridType _e_gridtype)
  (bind _actor (Default|GetObjectfromPool (Variables|Default|GetObjectPoolManager) (Utilities|Select :Index _e_gridtype :NewEnumerator0 "/Game/Resource/BP/Grid/Path/BP_GridPath.BP_GridPath_C" :NewEnumerator1 "/Game/Resource/BP/Grid/Monster/BP_GridMonster.BP_GridMonster_C" :NewEnumerator2 "/Game/Resource/BP/Grid/Special/BP_GridSpecialSpot.BP_GridSpecialSpot_C") Location "0, 0, 0"))
  (bind _asbp_grid (Utilities|Casting|CastToBP_Grid _actor)
    (:then
      (Variables|/Game/Resource/BP/Grid/BP_Grid.BP_Grid_C|SetE_GridType _asbp_grid (LocalVariables|GetTempGridType))
      (return _asbp_grid))
    (:CastFailed
      (return 0))))

(fn Move
  (bind _firstgridlocation (Variables|Cell|GetFirstGridLocation))
  (Math|Integer|IncrementInt (Variables|Default|GetTotalStep)
    (:%20%20
      (Utilities|Array|Clear (LocalVariables|GetTempGridLocations))
      (for (_array_element _array_index) (Variables|Cell|GetGrids)
        (Utilities|Array|SetArrayElem (LocalVariables|GetTempGridLocations) _array_index (Transformation|GetActorLocation _array_element) true)
        (if (> _array_index 0)
          (Utilities|Array|SetArrayElem (Variables|Cell|GetGrids) (- _array_index 1) _array_element)
          (if (== (- _array_index 1) (Variables|Default|GetPlayerSpot))
            (Rendering|SetVisibility (Variables|/Game/Resource/Character/Player/BP_Player.BP_Player_C|GetPlayerSprite (Variables|Default|GetAs%20BP%20Player)) (Utilities|Enum|Equal(Enum) (Variables|/Game/Resource/BP/Grid/BP_Grid.BP_Grid_C|GetE_GridType _array_element) "NewEnumerator0") false))
          (else
            (Default|ReturnObjecttoPool (Variables|Default|GetObjectPoolManager) (Utilities|Array|Get(acopy) (Variables|Cell|GetGrids))))))
      (bind _asbp_grid (CallFunction|SpawnRandomGrid (Math|Vector|MakeVector (+ (* (Utilities|Array|LastIndex (Variables|Cell|GetGrids)) 50) (.x _firstgridlocation)) (.y _firstgridlocation) (.z _firstgridlocation))))
      (Utilities|Array|SetArrayElem (Variables|Cell|GetGrids) (- (Variables|Cell|GetMaxGridCount) 1) _asbp_grid)
      (for (_array_element_2 _array_index_2) (Variables|Cell|GetGrids)
        (Transformation|SetActorLocation _array_element_2 (Utilities|Array|Get(acopy) (LocalVariables|GetTempGridLocations) _array_index_2) false false))
      (CallFunction|CompleteCards)
      (Utilities|FlowControl|Sequence
        (:then_0
          (bind _asbp_grid_special_spot (Utilities|Casting|CastToBP_GridSpecialSpot (Utilities|Array|Get(acopy) (Variables|Cell|GetGrids) (Variables|Default|GetPlayerSpot))))
          (Default|Show/HideSpotOption (Variables|Default|GetWBP_Game) true (Variables|/Game/Resource/BP/Grid/Special/BP_GridSpecialSpot.BP_GridSpecialSpot_C|GetSpotID _asbp_grid_special_spot))
          (CallFunction|AddStory (Utilities|String|ToString(Text) (Variables|/Game/Resource/BP/Grid/Special/BP_GridSpecialSpot.BP_GridSpecialSpot_C|GetSpot%20Description _asbp_grid_special_spot))))
        (:then_1
          (bind _asbp_grid_monster (Utilities|Casting|CastToBP_GridMonster (Utilities|Array|Get(acopy) (Variables|Cell|GetGrids) (Variables|Default|GetPlayerSpot))))
          (CallFunction|AddStory (Utilities|String|Append "你遇到了" (Utilities|String|ToString(Text) (Variables|/Game/Resource/BP/Grid/Monster/BP_GridMonster.BP_GridMonster_C|GetMonster%20Name _asbp_grid_monster)))))))))

(fn MonsterAction
  (bind _asbp_grid_monster (Utilities|Casting|CastToBP_GridMonster (Utilities|Array|Get(acopy) (Variables|Cell|GetGrids) (Variables|Default|GetPlayerSpot))))
  (if (not (Variables|/Game/Resource/BP/Grid/Monster/BP_GridMonster.BP_GridMonster_C|GetIsDie _asbp_grid_monster))
    (CallFunction|AddStory (Utilities|String|Append "你被" (Utilities|String|ToString(Text) (Variables|/Game/Resource/BP/Grid/Monster/BP_GridMonster.BP_GridMonster_C|GetMonster%20Name _asbp_grid_monster)) "攻击了," (select (>= (Utilities|Array|FindItem (Variables|/Game/Resource/Character/Player/BP_Player.BP_Player_C|GetSpecialCards (Variables|Default|GetAs%20BP%20Player)) "C_103") 0) (Utilities|String|Append "反弹咒语为你弹反了" (Utilities|String|ToString(Integer) (Math|Float|Truncate (Variables|/Game/Resource/BP/Grid/Monster/BP_GridMonster.BP_GridMonster_C|GetAttackPower _asbp_grid_monster))) "点伤害") (Utilities|String|Append "受到了" (Utilities|String|ToString(Integer) (Math|Float|Truncate (Variables|/Game/Resource/BP/Grid/Monster/BP_GridMonster.BP_GridMonster_C|GetAttackPower _asbp_grid_monster))) "点伤害"))))
    (Default|Attack _asbp_grid_monster (select (>= (Utilities|Array|FindItem (Variables|/Game/Resource/Character/Player/BP_Player.BP_Player_C|GetSpecialCards (Variables|Default|GetAs%20BP%20Player)) "C_103") 0) _asbp_grid_monster (Variables|Default|GetAs%20BP%20Player)) (Variables|/Game/Resource/BP/Grid/Monster/BP_GridMonster.BP_GridMonster_C|GetAttackPower _asbp_grid_monster))))

(fn UseCurrentSpot
  (bind _asbp_grid_special_spot (Utilities|Casting|CastToBP_GridSpecialSpot (Utilities|Array|Get(acopy) (Variables|Cell|GetGrids) (Variables|Default|GetPlayerSpot))))
  (Default|Used _asbp_grid_special_spot))

(fn SetStory
  (Default|SetText (Variables|/Game/Resource/BP/WBP/Game/WBP_Game.WBP_Game_C|GetWBP_GameProcess (Variables|Default|GetWBP_Game)) (Variables|Default|GetStory)))

(fn AddStory
  (params (Story :type String))
  (Variables|Default|SetStory (Utilities|String|Append (Variables|Default|GetStory) Story "\\n"))
  (CallFunction|SetStory))